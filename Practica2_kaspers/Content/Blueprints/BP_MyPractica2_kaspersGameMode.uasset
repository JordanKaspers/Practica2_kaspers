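; Game mode that runs a timed level and returns the game to the Menu level when time runs out.
; BeginPlay fills a projectile pool, and each Tick recomputes the whole seconds left by subtracting elapsed game time from the time limit.
; GetTimeLeft exposes the remaining time, while a disconnected branch that would pause the game through the player character never runs.
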(event EventBeginPlay
  (Class|MyPractica2KaspersGameMode|PopulateProjectilePool))

(event EventTick
  (params (DeltaSeconds :type Float%20%28single-precision%29))
  (CallFunction|Countdown))

(fn ConstructionScript)

(fn Countdown
  (bind _returnvalue (Utilities|Time|GetTimeSeconds))
  (bind _timelimit (Variables|Default|GetTimeLimit))
  (bind _returnvalue_2 (- _timelimit _returnvalue))
  (if (> _returnvalue_2 0.0)
    (Variables|Default|SetTimeLeft (Math|Float|Floor _returnvalue_2))
    (else
      (Game|OpenLevel(byName) "Menu"))))

(fn GetTimeLeft
  (return (Variables|Default|GetTimeLeft)))