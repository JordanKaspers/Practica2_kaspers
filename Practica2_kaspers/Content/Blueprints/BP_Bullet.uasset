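; BP_Bullet is a bullet actor that makes noise when it reaches the player.
; It plays its audio on spawn.
; When its collision component overlaps BP_PlayerCharacter, it reports a noise event at the player's location with itself as instigator, limited to SoundRadius.
; It also draws a short-lived debug sphere of that radius around the bullet; the hit event is empty, and no damage or movement logic appears in the graphs.
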(event OnComponentHit(CollisionComp)
  (params (HitComponent :type Primitive%20Component%20Object%20Reference) (OtherActor :type Actor%20Object%20Reference) (OtherComp :type Primitive%20Component%20Object%20Reference) (NormalImpulse :type Vector :default "0, 0, 0") (Hit :type Hit%20Result%20Structure%20%28by%20ref%29)))

(event OnComponentBeginOverlap(CollisionComp)
  (params (OverlappedComponent :type Primitive%20Component%20Object%20Reference) (OtherActor :type Actor%20Object%20Reference) (OtherComp :type Primitive%20Component%20Object%20Reference) (OtherBodyIndex :type Integer) (bFromSweep :type Boolean) (SweepResult :type Hit%20Result%20Structure%20%28by%20ref%29))
  (bind _asbp_player_character (Utilities|Casting|CastToBP_PlayerCharacter OtherActor))
  (Class|AISenseHearing|ReportNoiseEvent (Transformation|GetActorLocation _asbp_player_character) 1.0 self (Variables|Default|GetSoundRadius) "None")
  (Rendering|Debug|DrawDebugSphere (Transformation|GetActorLocation) (Variables|Default|GetSoundRadius) 12 "(R=1.000000,G=0.000000,B=0.024906,A=1.000000)" 2.0 0.2))

(event EventBeginPlay
  (Audio|Components|Audio|Play (Variables|Default|GetAudio) 0.0))

(event Collision|EventActorBeginOverlap
  (params (OtherActor :type Actor%20Object%20Reference)))

(event EventTick
  (params (DeltaSeconds :type Float%20%28single-precision%29)))

(fn ConstructionScript)