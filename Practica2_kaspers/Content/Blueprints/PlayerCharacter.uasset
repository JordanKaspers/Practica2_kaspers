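; Player character for a stealth game, with sneak, crouch, run and throw inputs and a Health value.
; Movement inputs set walk speed and state flags, which Tick turns into AI noise reports each frame, including while standing still.
; Bullet-tagged capsule overlaps reduce Health, while Enemy-tagged DeathArea overlaps zero it.
; Throw plays a montage; separate functions spawn the projectile and particles, with no caller in this graph.
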(event OnComponentBeginOverlap(CapsuleComponent)
  (params (OverlappedComponent :type Primitive%20Component%20Object%20Reference) (OtherActor :type Actor%20Object%20Reference) (OtherComp :type Primitive%20Component%20Object%20Reference) (OtherBodyIndex :type Integer) (bFromSweep :type Boolean) (SweepResult :type Hit%20Result%20Structure%20%28by%20ref%29))
  (if (Actor|ActorHasTag OtherActor "Bullet")
    (if (<= (Variables|Default|GetHealth) 0)
      (Variables|Default|SetHealth 0)
      (else
        (Variables|Default|SetHealth (- (Variables|Default|GetHealth) 25))))))

(event OnComponentBeginOverlap(DeathArea)
  (params (OverlappedComponent :type Primitive%20Component%20Object%20Reference) (OtherActor :type Actor%20Object%20Reference) (OtherComp :type Primitive%20Component%20Object%20Reference) (OtherBodyIndex :type Integer) (bFromSweep :type Boolean) (SweepResult :type Hit%20Result%20Structure%20%28by%20ref%29))
  (if (Actor|ActorHasTag OtherActor "Enemy")
    (Variables|Default|SetHealth 0)))

(event Custom|Throw
  (Animation|PlayAnimMontage "/Game/MyMannequin/Animations/Player/Throw_AnimMontage.Throw_AnimMontage" 1.0 "None"))

(event EventTick
  (params (DeltaSeconds :type Float%20%28single-precision%29))
  (Utilities|FlowControl|Sequence
    (:then_0
      (if (Variables|Default|GetRunning)
        (Class|AISenseHearing|ReportNoiseEvent (Transformation|GetActorLocation) (Variables|Default|GetRunVolume) self (Variables|Default|GetSoundRadius) "None")))
    (:then_1
      (if (Variables|Default|GetCrouching)
        (Class|AISenseHearing|ReportNoiseEvent (Transformation|GetActorLocation) (Variables|Default|GetCrouchVolume) self (Variables|Default|GetSoundRadius) "None")))
    (:then_2
      (if (Math|Boolean|ANDBoolean (Pawn|Components|CharacterMovement|IsWalking (Variables|Character|GetCharacterMovement)) (not (Variables|Default|GetSneaking)) (not (Variables|Default|GetCrouching)))
        (Class|AISenseHearing|ReportNoiseEvent (Transformation|GetActorLocation) (Variables|Default|GetWalkVolume) self (Variables|Default|GetSoundRadius) "None")))))

(event EventBeginPlay
  (bind _output_get (Variables|/Script/Engine.CharacterMovementComponent|SetMaxWalkSpeed (Variables|Character|GetCharacterMovement) (Variables|Default|GetMaxWalkSpeed)))
  (Variables|Default|SetSpeed _output_get))

(event Input|ActionEvents|InputActionRun
  (params (Key :type Key%20Structure :default "AnyKey"))
  (bind _charactermovement (Variables|Character|GetCharacterMovement))
  (:Pressed
    (Variables|Default|SetRunning true)
    (bind _output_get (Variables|/Script/Engine.CharacterMovementComponent|SetMaxWalkSpeed _charactermovement (Variables|Default|GetRunSpeed)))
    (Variables|Default|SetSpeed _output_get))
  (:Released
    (Variables|Default|SetRunning false)
    (bind _output_get_2 (Variables|/Script/Engine.CharacterMovementComponent|SetMaxWalkSpeed _charactermovement (Variables|Default|GetMaxWalkSpeed)))
    (Variables|Default|SetSpeed _output_get_2)))

(event Input|ActionEvents|InputActionSneak
  (params (Key :type Key%20Structure :default "AnyKey"))
  (bind _charactermovement (Variables|Character|GetCharacterMovement))
  (:Pressed
    (Variables|Default|SetSneaking true)
    (bind _output_get (Variables|/Script/Engine.CharacterMovementComponent|SetMaxWalkSpeed _charactermovement (Variables|Default|GetSneakSpeed))))
  (:Released
    (Variables|Default|SetSneaking false)
    (bind _output_get_2 (Variables|/Script/Engine.CharacterMovementComponent|SetMaxWalkSpeed _charactermovement (Variables|Default|GetMaxWalkSpeed)))
    (Variables|Default|SetSpeed _output_get_2)))

(event Input|ActionEvents|InputActionCrouch
  (params (Key :type Key%20Structure :default "AnyKey"))
  (bind _charactermovement (Variables|Character|GetCharacterMovement))
  (:Pressed
    (Variables|Default|SetCrouching true)
    (Character|Crouch)
    (bind _output_get (Variables|/Script/Engine.CharacterMovementComponent|SetMaxWalkSpeed _charactermovement (Variables|Default|GetCrouchSpeed)))
    (Variables|Default|SetSpeed _output_get))
  (:Released
    (Variables|Default|SetCrouching false)
    (Character|UnCrouch)
    (bind _output_get_2 (Variables|/Script/Engine.CharacterMovementComponent|SetMaxWalkSpeed _charactermovement (Variables|Default|GetMaxWalkSpeed)))
    (Variables|Default|SetSpeed _output_get_2)))

(event Input|ActionEvents|InputActionThrow
  (params (Key :type Key%20Structure :default "AnyKey"))
  (:Pressed
    (Variables|Default|SetThrowing true)
    (CallFunction|Throw))
  (:Released
    (Variables|Default|SetThrowing false)))

(fn ConstructionScript)

(fn SpawnThrowingParticles
  (params (SpawnPoint :type Transform))
  (bind (_location _rotation) (Math|Transform|BreakTransform SpawnPoint))
  (Effects|SpawnEmitteratLocation "/Game/Particles/PS_SpawnProjectile.PS_SpawnProjectile" _location _rotation))

(fn SpawnProjectile
  (params (Transform :type Transform))
  (Game|SpawnActorfromClass "/Game/Blueprints/BP_Projectile.BP_Projectile_C" Transform "Undefined" 0 0))

(fn GetHealth
  (return (Variables|Default|GetHealth)))