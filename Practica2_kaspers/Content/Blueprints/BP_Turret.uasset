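; BP_Turret is a turret Blueprint that sets up its aiming and pool reference when play begins.
; On BeginPlay it initialises a TurretAiming component with its Barrel and Dome parts.
; It then casts the game mode to MyPractica2_kaspersGameMode, fetches a pool from it, stores it via SetPool, and starts its Audio component playing.
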(event EventBeginPlay
  (Class|TurretAimingComponent|Initialise (Variables|Default|GetTurretAiming) (Variables|Default|GetBarrel) (Variables|Default|GetDome))
  (bind _asmy_practica_2_kaspers_game_mode (Utilities|Casting|CastToMyPractica2_kaspersGameMode (Game|GetGameMode)))
  (bind _returnvalue (Class|MyPractica2KaspersGameMode|GetPool _asmy_practica_2_kaspers_game_mode))
  (Class|Turret|SetPool self _returnvalue)
  (Audio|Components|Audio|Play (Variables|Default|GetAudio) 0.0))

(fn ConstructionScript)