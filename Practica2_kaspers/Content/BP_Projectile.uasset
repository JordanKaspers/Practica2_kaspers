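; Projectile actor that makes a noise for AI hearing where it strikes.
; On BeginPlay it launches itself through LaunchProjectile at a fixed speed.
; A collision component hit reports a noise event at the actor's location with SoundRadius as range, instigated by itself, and draws a debug sphere of that radius.
; Lifespan and velocity nodes are left unconnected, so the graph never destroys the projectile.
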(event OnComponentHit(CollisionComp)
  (params (HitComponent :type Primitive%20Component%20Object%20Reference) (OtherActor :type Actor%20Object%20Reference) (OtherComp :type Primitive%20Component%20Object%20Reference) (NormalImpulse :type Vector :default "0, 0, 0") (Hit :type Hit%20Result%20Structure%20%28by%20ref%29))
  (Class|AISenseHearing|ReportNoiseEvent (Transformation|GetActorLocation) 1.0 self (Variables|Default|GetSoundRadius) "None")
  (Rendering|Debug|DrawDebugSphere (Transformation|GetActorLocation) (Variables|Default|GetSoundRadius) 12 "(R=1.000000,G=0.000000,B=0.024906,A=1.000000)" 2.0 0.2))

(event EventBeginPlay
  (Class|Projectile|LaunchProjectile 2e+03))

(event Collision|EventActorBeginOverlap
  (params (OtherActor :type Actor%20Object%20Reference)))

(event EventTick
  (params (DeltaSeconds :type Float%20%28single-precision%29)))

(event Collision|EventHit
  (params (MyComp :type Primitive%20Component%20Object%20Reference) (Other :type Actor%20Object%20Reference) (OtherComp :type Primitive%20Component%20Object%20Reference) (bSelfMoved :type Boolean) (HitLocation :type Vector) (HitNormal :type Vector :default "0, 0, 0") (NormalImpulse :type Vector :default "0, 0, 0") (Hit :type Hit%20Result%20Structure%20%28by%20ref%29)))

(fn ConstructionScript)